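; BP_cat_GM is the game manager for an endless-runner style game, handling spawning, distance scoring and game over.
; BeginPlay creates the GameOver_HUD widget and starts a looping timer that randomly spawns either an enemy or an obstacle at a fixed point.
; Tick accumulates distance at a constant rate and updates the HUD until the game ends.
; GameOver stops scoring, shows the restart button and cursor, then pauses after a short delay.
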(event `self.ReceiveBeginPlay`
  (set `self.GameisOver` false)
  (bind _returnvalue (`|CreateWidget` "/Game/Blueprint/GameOver_HUD.GameOver_HUD_C" (`GameplayStatics.GetPlayerController` 0)))
  (bind _output_get (set `self.Game HUD` _returnvalue))
  (`UserWidget.AddToViewport` _output_get 0)
  (`KismetSystemLibrary.K2_SetTimerDelegate` (delegate `SpawnRandom`) 0.75 true))

(event `SpawnRandom`
  (`|SpawnActorFromClass` (select `bool` (`KismetMathLibrary.RandomBool`) :`false` "/Game/Blueprint/BP_Obstacles.BP_Obstacles_C" :`true` "/Game/Blueprint/BP_Enemies.BP_Enemies_C" :!type "Actor Class Reference") (`KismetMathLibrary.MakeTransform` (1400.0 0.0 -170.0)) "Undefined" "OverrideRootScale" null null))

(event `self.ReceiveTick`
  (params (DeltaSeconds :type "Float (single-precision)"))
  (if (not (`self.GameisOver`))
    (bind _output_get (set `self.TotalDistance` (+ (`self.TotalDistance`) (* DeltaSeconds 1400.0))))
    (`/Game/Blueprint/GameOver_HUD.Update Distance Text` (`self.Game HUD`) (/ _output_get 100.0))))

(event `Game Over`
  (set `self.GameisOver` true)
  (`/Game/Blueprint/GameOver_HUD.Show restart button` (`self.Game HUD`))
  (set `PlayerController.bShowMouseCursor` true (`GameplayStatics.GetPlayerController` 0))
  (`KismetSystemLibrary.Delay` 0.75)
  (`GameplayStatics.SetGamePaused` true))

(fn `UserConstructionScript`)